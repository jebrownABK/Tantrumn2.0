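; BP_Explosion is a proximity-triggered explosion actor that goes off when a BP_Player overlaps its box.
; The overlap activates the particle system, whose activation event plays the explosion sound at its location.
; Nested distance checks against the player then gate a delayed self-destruct, so the actor is destroyed only if the player is within the innermost radius.
; The construction script sets the trigger box's transform from BoxTransform.
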(event `self.ParticleSystem.OnComponentActivated`
  (params (Component :type "ActorComponent Object Reference") (bReset :type Boolean))
  (`GameplayStatics.PlaySoundAtLocation` "/Game/StarterContent/Audio/Explosion_Cue.Explosion_Cue" (`SceneComponent.K2_GetComponentLocation` (`self.ParticleSystem`)) (struct) 1.0 1.0 0.0 null null null)
  (bind _asbp_player (cast `/Game/Tantrumn/Blueprints/Characters/BP_Player` (`GameplayStatics.GetPlayerCharacter` 0)))
  (bind _returnvalue (`self.GetDistanceTo` _asbp_player))
  (if (<= _returnvalue 700.0)
    (if (<= _returnvalue 500.0)
      (if (<= _returnvalue 400.0)
        (`KismetSystemLibrary.Delay` 3.0)
        (`self.K2_DestroyActor`)))))

(event `self.Box.OnComponentBeginOverlap`
  (params (OverlappedComponent :type "PrimitiveComponent Object Reference") (OtherActor :type "Actor Object Reference") (OtherComp :type "PrimitiveComponent Object Reference") (OtherBodyIndex :type Integer) (bFromSweep :type Boolean) (SweepResult :type "HitResult Structure (by ref)"))
  (cast `/Game/Tantrumn/Blueprints/Characters/BP_Player` OtherActor)
  (`ActorComponent.Activate` (`self.ParticleSystem`) false))

(fn `UserConstructionScript`
  (`SceneComponent.K2_SetRelativeTransform` (`self.Box`) (`self.Box Transform`) false false))