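; Exploding bomb actor that moves along its forward vector until it reaches a length limit; no explosion logic is present.
; BeginPlay runs a debug-drawn box trace against WorldStatic and replaces Length with any hit distance.
; Tick applies swept, Speed-scaled offsets until the length check sets Stop.
; Both the trace end and travelled-length check multiply vectors component-wise instead of adding or subtracting them.
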(event `self.ReceiveBeginPlay`
  (bind _startlocation (`self.startLocation`))
  (set `self.startLocation` (`self.K2_GetActorLocation`))
  (bind (_outhit _returnvalue) (`KismetSystemLibrary.BoxTraceSingleForObjects` :`Start` _startlocation :`End` (* _startlocation (* (`self.GetActorForwardVector`) (`self.length`))) :`HalfSize` (20.0 20.0 20.0) :`ObjectTypes` (`|MakeArray` "ObjectTypeQuery1" :!type "EObjectTypeQuery Enum") :`DrawDebugType` "ForDuration"))
  (if _returnvalue
    (set `self.length` (`.Distance` (`GameplayStatics.BreakHitResult` _outhit)))))

(event `self.ReceiveTick`
  (params (DeltaSeconds :type "Float (single-precision)"))
  (if (not (`self.stop`))
    (`self.K2_AddActorWorldOffset` (* (`self.GetActorForwardVector`) (* DeltaSeconds (`self.speed`))) true)
    (if (>= (`KismetMathLibrary.VSize` (* (`self.startLocation`) (`self.K2_GetActorLocation`))) (`self.length`))
      (set `self.stop` true))))

(fn `UserConstructionScript`)